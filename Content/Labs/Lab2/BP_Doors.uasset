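; BP_Doors is an interactable, key-locked sliding door for the maze lab.
; On Interact it compares its KeyNumber to the Keys value on the GM_Maze game mode, cached at BeginPlay, and requires an exact match.
; A match plays a Timeline that lerps the door sideways; otherwise a warning prints.
; The construction script picks the door material from KeyNumber, and GetInteractState always returns false.
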(event EventBeginPlay
  (bind _asgm_maze (Utilities|Casting|CastToGM_Maze (Game|GetGameMode)))
  (Variables|Default|SetAs%20GM%20Maze _asgm_maze))

(event EventInteract
  (if (== (Variables|Default|GetKeyNumber) (Variables|/Game/Labs/Lab2/GM_Maze.GM_Maze_C|GetKeys (Variables|Default|GetAs%20GM%20Maze)))
    (bind _doorturn (Timeline|Timeline Play)
      (:Update
        (Transformation|SetRelativeLocation (Variables|Default|GetDoor) (Math|Vector|Lerp(Vector) "0, 0, 0" "0.000000,-500.000000,0.000000" _doorturn) false false)
        (Utilities|FlowControl|Delay 5.0)))
    (else
      (Development|PrintString "YOU DON'T HAVE THE REQUIRED KEY TO OPEN THIS DOOR!!"))))

(fn ConstructionScript
  (bind _door (Variables|Default|GetDoor))
  (switch int (Variables|Default|GetKeyNumber)
    (:0
      (Rendering|Material|SetMaterial _door 0 "/Engine/MapTemplates/Materials/BasicAsset03.BasicAsset03"))
    (:1
      (Rendering|Material|SetMaterial _door 0 "/Engine/MapTemplates/Materials/BasicAsset01.BasicAsset01"))))

(fn GetInteractState
  (return false))