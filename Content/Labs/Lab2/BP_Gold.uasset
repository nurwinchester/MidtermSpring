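; Interactable gold pickup that adds a random amount to the GoldAmount of the GM_Maze game mode.
; The construction script rolls the value, then runs the CreateMesh macro against gold thresholds to add static meshes with random XY offsets and heights.
; Interact uses the game mode reference cached on BeginPlay to add the gold, prints the new total and destroys the actor.
; GetInteractState always returns false.
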(event EventBeginPlay
  (bind _asgm_maze (Utilities|Casting|CastToGM_Maze (Game|GetGameMode)))
  (Variables|Default|SetAs%20GM%20Maze _asgm_maze))

(event EventInteract
  (bind _output_get (Variables|/Game/Labs/Lab2/GM_Maze.GM_Maze_C|SetGoldAmount (Variables|Default|GetAs%20GM%20Maze) (+ (Variables|Default|GetGold) (Variables|/Game/Labs/Lab2/GM_Maze.GM_Maze_C|GetGoldAmount (Variables|Default|GetAs%20GM%20Maze)))))
  (Development|PrintString (Utilities|String|ToString(Integer) _output_get))
  (Actor|DestroyActor))

(fn ConstructionScript
  (Variables|Default|SetGold (Math|Random|RandomIntegerinRange 1 99))
  (Utilities|CreateMesh (<= (Variables|Default|GetGold) 26)
    (:Out
      _)
    (:False
      _))
  (Utilities|CreateMesh (<= (Variables|Default|GetGold) 76)
    (:Out
      _)
    (:False
      _))
  (Utilities|CreateMesh (<= (Variables|Default|GetGold) 100)))

(fn GetInteractState
  (return false))