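; BP_Keys is a spinning key pickup for a maze, identified by a key number.
; Its construction script picks the key mesh's material from that number, and Tick rotates the actor around its roll axis.
; On Interact it writes the number to the GM_Maze game mode's Keys value, replacing any previous one, prints the acquired key's name and destroys itself.
; GetInteractState always returns false.
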(event EventBeginPlay
  (bind _asgm_maze (Utilities|Casting|CastToGM_Maze (Game|GetGameMode)))
  (Variables|Default|SetAs%20GM%20Maze_ _asgm_maze))

(event EventTick
  (params (DeltaSeconds :type Float%20%28single-precision%29))
  (Transformation|AddActorLocalRotation (Math|Rotator|MakeRotator (* DeltaSeconds (Variables|Default|GetRotation)) 0.0 0.0) false false))

(event EventInteract
  (bind _output_get (Variables|/Game/Labs/Lab2/GM_Maze.GM_Maze_C|SetKeys (Variables|Default|GetAs%20GM%20Maze_) (Variables|Default|GetKeyNumber)))
  (Development|PrintString (Utilities|String|Append (Utilities|Array|Get(acopy) (Variables|Default|GetNames) _output_get) " Key Aquired"))
  (Actor|DestroyActor))

(fn ConstructionScript
  (bind _key (Variables|Default|GetKey))
  (switch int (Variables|Default|GetKeyNumber)
    (:0
      (Rendering|Material|SetMaterial _key 0 "/Engine/MapTemplates/Materials/BasicAsset03.BasicAsset03"))
    (:1
      (Rendering|Material|SetMaterial _key 0 "/Engine/MapTemplates/Materials/BasicAsset01.BasicAsset01"))))

(fn GetInteractState
  (return false))