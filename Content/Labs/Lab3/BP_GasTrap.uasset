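; BP_GasTrap is a gas trap actor that damages the player over time while they stand inside it.
; Cube overlap starts and clears a looping timer by function name, whose Dot event repeatedly applies negative HealthUpdate to the player character.
; On BeginPlay it caches the player character and passes DP_Trap_Event to its AssignDPTrap, destroying itself when the received value matches its TrapType.
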(event OnComponentBeginOverlap(Cube)
  (params (OverlappedComponent :type Primitive%20Component%20Object%20Reference) (OtherActor :type Actor%20Object%20Reference) (OtherComp :type Primitive%20Component%20Object%20Reference) (OtherBodyIndex :type Integer) (bFromSweep :type Boolean) (SweepResult :type Hit%20Result%20Structure%20%28by%20ref%29))
  (if (== OtherActor (Variables|Default|GetAs%20BP%20Third%20Person%20Character))
    (Utilities|Time|SetTimerbyFunctionName 0 "Dot" 0.1 true)))

(event OnComponentEndOverlap(Cube)
  (params (OverlappedComponent :type Primitive%20Component%20Object%20Reference) (OtherActor :type Actor%20Object%20Reference) (OtherComp :type Primitive%20Component%20Object%20Reference) (OtherBodyIndex :type Integer))
  (if (== OtherActor (Variables|Default|GetAs%20BP%20Third%20Person%20Character))
    (Utilities|Time|ClearTimerbyFunctionName 0 "Dot")))

(event Custom|Dot
  (Default|HealthUpdate (Variables|Default|GetAs%20BP%20Third%20Person%20Character) -1.0))

(event Custom|DP_Trap_Event
  (params (NewParam :type Enum_TrapType%20Enum :default "NewEnumerator0"))
  (if (Utilities|Enum|Equal(Enum) (Variables|Default|GetTrapType) NewParam)
    (Actor|DestroyActor)))

(event EventBeginPlay
  (bind _asbp_third_person_character (Utilities|Casting|CastToBP_ThirdPersonCharacter (Game|GetPlayerCharacter 0)))
  (bind _output_get (Variables|Default|SetAs%20BP%20Third%20Person%20Character _asbp_third_person_character))
  (EventDispatchers|AssignDPTrap _output_get (delegate Custom|DP_Trap_Event)))

(event Collision|EventActorBeginOverlap
  (params (OtherActor :type Actor%20Object%20Reference)))

(fn ConstructionScript)