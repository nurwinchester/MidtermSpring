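; BP_SpikeTrap is a spike trap that damages the player and can be disabled by trap type.
; Player overlap with ActivationBox plays a Timeline that moves the spike mesh along Z, while overlap with DamageBox reduces player health.
; It binds to the player character's DPTrap dispatcher at BeginPlay.
; A matching TrapType lowers the spikes, turns off both boxes' collision and destroys the Timeline, permanently disarming the trap.
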(event OnComponentBeginOverlap(DamageBox)
  (params (OverlappedComponent :type Primitive%20Component%20Object%20Reference) (OtherActor :type Actor%20Object%20Reference) (OtherComp :type Primitive%20Component%20Object%20Reference) (OtherBodyIndex :type Integer) (bFromSweep :type Boolean) (SweepResult :type Hit%20Result%20Structure%20%28by%20ref%29))
  (if (== OtherActor (Variables|Default|GetAs%20BP%20Third%20Person%20Character))
    (Default|HealthUpdate (Variables|Default|GetAs%20BP%20Third%20Person%20Character) -25.0)))

(event OnComponentBeginOverlap(ActivationBox)
  (params (OverlappedComponent :type Primitive%20Component%20Object%20Reference) (OtherActor :type Actor%20Object%20Reference) (OtherComp :type Primitive%20Component%20Object%20Reference) (OtherBodyIndex :type Integer) (bFromSweep :type Boolean) (SweepResult :type Hit%20Result%20Structure%20%28by%20ref%29))
  (if (== OtherActor (Variables|Default|GetAs%20BP%20Third%20Person%20Character))
    (Variables|Default|GetTimeline
      (:then
        (bind _newtrack_0 (Timeline|Timeline Play)
          (:Update
            (Transformation|SetRelativeLocation (Variables|Default|GetSpikeTrap_354EFE8E) (Math|Vector|MakeVector 0.0 0.0 _newtrack_0) false false))))
      (:else))))

(event Custom|DP_Trap_Event
  (params (NewParam :type Enum_TrapType%20Enum :default "NewEnumerator0"))
  (if (Utilities|Enum|Equal(Enum) (Variables|Default|GetTrapType) NewParam)
    (Transformation|SetRelativeLocation (Variables|Default|GetSpikeTrap_354EFE8E) "0.000000,0.000000,-165.000000" false false)
    (Collision|SetCollisionEnabled (Variables|Default|GetDamageBox) "NoCollision")
    (Components|DestroyComponent (Variables|Default|GetTimeline))))

(event EventBeginPlay
  (bind _asbp_third_person_character (Utilities|Casting|CastToBP_ThirdPersonCharacter (Game|GetPlayerCharacter 0)))
  (bind _output_get (Variables|Default|SetAs%20BP%20Third%20Person%20Character _asbp_third_person_character))
  (EventDispatchers|AssignDPTrap _output_get (delegate Custom|DP_Trap_Event)))

(event Collision|EventActorBeginOverlap
  (params (OtherActor :type Actor%20Object%20Reference)))

(event EventTick
  (params (DeltaSeconds :type Float%20%28single-precision%29)))

(fn ConstructionScript)