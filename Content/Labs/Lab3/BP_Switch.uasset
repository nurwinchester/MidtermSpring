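; BP_Switch is an interactable switch that triggers traps of a set TrapType through the player character.
; BeginPlay caches the BP_ThirdPersonCharacter, and Interact passes TrapType to its CallDPTrap, so the switch holds no direct trap references.
; The construction script writes the enum name to a text render as a label, and GetInteractState always returns false.
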(event EventBeginPlay
  (bind _asbp_third_person_character (Utilities|Casting|CastToBP_ThirdPersonCharacter (Game|GetPlayerCharacter 0)))
  (Variables|Default|SetAs%20BP%20Third%20Person%20Character _asbp_third_person_character))

(event EventInteract
  (Default|CallDPTrap (Variables|Default|GetAs%20BP%20Third%20Person%20Character) (Variables|Default|GetTrapType)))

(fn ConstructionScript
  (Rendering|Components|TextRender|SetText (Variables|Default|GetTextRender) (Utilities|Text|ToText(String) (Utilities|String|EnumtoString (Variables|Default|GetTrapType)))))

(fn GetInteractState
  (return false))